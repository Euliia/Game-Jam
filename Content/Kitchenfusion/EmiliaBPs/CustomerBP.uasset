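; Customer actor for a kitchen game that places a randomly generated burger-style order.
; On BeginPlay it picks a random idle-named skeletal mesh, then fills its Order array with a random number of randomly chosen, possibly repeated ingredients.
; The order is debug-printed and shown on a TextRender as one string joined without separators.
; OrderIsCorrect asks the handler reference to remove a customer; no order checking happens here.
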(event Custom|OrderIsCorrect
  (Default|Removecustomer (Variables|Default|GetHandlerRef)))

(event EventBeginPlay
  (Class|SkinnedMeshComponent|SetSkeletalMesh (Variables|Default|GetSkeletalMesh) (.OutItem (Utilities|Array|Random (Utilities|Array|MakeArray "/Game/customermodels/character_model_animation/Neutral_Idle1.Neutral_Idle1" "/Game/customermodels/character_model_animation/Neutral_Idle2.Neutral_Idle2" "/Game/customermodels/character_model_animation/Neutral_Idle3.Neutral_Idle3" "/Game/customermodels/character_model_animation/Neutral_Idle4.Neutral_Idle4" "/Game/customermodels/character_model_animation/Neutral_Idle5.Neutral_Idle5"))) true)
  (for _index (range 0 (Math|Random|RandomInteger 7))
    (Utilities|Array|Add (Variables|Default|GetOrder) (.OutItem (Utilities|Array|Random (Utilities|Array|MakeArray "Bun" "Lettuce" "Patty" "Tomato" "Onion" "Pickles" "Sauce" "Cheese")))))
  (for _array_element (Variables|Default|GetOrder)
    (Development|PrintString _array_element))
  (Rendering|Components|TextRender|SetText (Variables|Default|GetTextRender) (Utilities|Text|ToText(String) (Utilities|String|JoinStringArray (Variables|Default|GetOrder) " 
"))))

(fn ConstructionScript)