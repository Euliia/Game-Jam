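; ItemBP is a pickup for burger ingredients such as bun, patty and cheese in the kitchen game.
; The construction script picks a placeholder-looking bunker food mesh from the item's Name, falling back to a water jug.
; Sphere overlap with the first-person character opens a gate for the E key.
; Pickup prints the Name and adds it and MyType to the character's list, leaving the item in the world.
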(event OnComponentBeginOverlap(Sphere)
  (params (OverlappedComponent :type Primitive%20Component%20Object%20Reference) (OtherActor :type Actor%20Object%20Reference) (OtherComp :type Primitive%20Component%20Object%20Reference) (OtherBodyIndex :type Integer) (bFromSweep :type Boolean) (SweepResult :type Hit%20Result%20Structure%20%28by%20ref%29))
  (Utilities|Casting|CastToBP_FirstPersonCharacterE OtherActor)
  (Utilities|FlowControl|Gate true) ; enters at Open
)

(event OnComponentEndOverlap(Sphere)
  (params (OverlappedComponent :type Primitive%20Component%20Object%20Reference) (OtherActor :type Actor%20Object%20Reference) (OtherComp :type Primitive%20Component%20Object%20Reference) (OtherBodyIndex :type Integer))
  (Utilities|Casting|CastToBP_FirstPersonCharacterE OtherActor)
  (Utilities|FlowControl|Gate true) ; enters at Close
)

(event Custom|Pickup
  (Development|PrintString (Variables|Default|GetName))
  (bind _asbp_first_person_character (Utilities|Casting|CastToBP_FirstPersonCharacterE (Game|GetPlayerCharacter 0)))
  (Default|AddtoList _asbp_first_person_character (Variables|Default|GetName) (Variables|Default|GetMyType)))

(event Input|KeyboardEvents|E
  (params (Key :type Key%20Structure))
  (:Pressed
    (Utilities|FlowControl|Gate true
      (:Exit
        (Development|PrintString (Variables|Default|GetName))
        (bind _asbp_first_person_character (Utilities|Casting|CastToBP_FirstPersonCharacterE (Game|GetPlayerCharacter 0)))
        (Default|AddtoList _asbp_first_person_character (Variables|Default|GetName) (Variables|Default|GetMyType))))))

(fn ConstructionScript
  (switch string (Variables|Default|GetName)
    (:Default
      (Components|StaticMesh|SetStaticMesh (Variables|Default|GetItem) "/Game/EF_Barbra/Meshes/BunkerFoodWaterJug_a.BunkerFoodWaterJug_a"))
    (:Bun
      (Components|StaticMesh|SetStaticMesh (Variables|Default|GetItem) "/Game/EF_Barbra/Meshes/BunkerFoodCan_c.BunkerFoodCan_c"))
    (:Lettuce
      (Components|StaticMesh|SetStaticMesh (Variables|Default|GetItem) "/Game/EF_Barbra/Meshes/BunkerFoodCan_b.BunkerFoodCan_b"))
    (:Patty
      (Components|StaticMesh|SetStaticMesh (Variables|Default|GetItem) "/Game/EF_Barbra/Meshes/BunkerFoodCan_a.BunkerFoodCan_a"))
    (:Tomato
      (Components|StaticMesh|SetStaticMesh (Variables|Default|GetItem) "/Game/EF_Barbra/Meshes/BunkerFoodCereal_a.BunkerFoodCereal_a"))
    (:Onion
      (Components|StaticMesh|SetStaticMesh (Variables|Default|GetItem) "/Game/EF_Barbra/Meshes/BunkerFoodCereal_b.BunkerFoodCereal_b"))
    (:Pickles
      (Components|StaticMesh|SetStaticMesh (Variables|Default|GetItem) "/Game/EF_Barbra/Meshes/BunkerFoodJar_a.BunkerFoodJar_a"))
    (:Sauce
      (Components|StaticMesh|SetStaticMesh (Variables|Default|GetItem) "/Game/EF_Barbra/Meshes/BunkerFoodJar_b.BunkerFoodJar_b"))
    (:Cheese
      (Components|StaticMesh|SetStaticMesh (Variables|Default|GetItem) "/Game/EF_Barbra/Meshes/BunkerFoodJar_c.BunkerFoodJar_c"))))